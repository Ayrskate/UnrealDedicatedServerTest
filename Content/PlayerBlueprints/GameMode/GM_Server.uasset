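; GM_Server is a game mode that tracks connected players and spawns their characters once more than one has joined.
; PostLogin fills the AllPlayers list, then a one-time pass spawns a ThirdPersonCharacter for each controller at a PlayerStart looked up by list index and possesses it.
; The first player's character is tagged "Instructor" and the others "Alumno" (student).
; Logout removes the controller from the list.
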(event `self.K2_PostLogin`
  (params (NewPlayer :type "PlayerController Object Reference"))
  (bind _allplayers (`self.AllPlayers`))
  (`KismetArrayLibrary.Array_Add` _allplayers NewPlayer)
  (if (> (`KismetArrayLibrary.Array_Length` _allplayers) 1)
    (`KismetSystemLibrary.PrintString` "Game can start!" true true (struct :`G` 0.66 :`B` 1.0 :`A` 1.0) 5.0)
    (`/Engine/EditorBlueprintResources/StandardMacros.DoOnce` false
      (:`Completed`
        (for (_array_element _array_index) (`self.AllPlayers`)
          (bind _returnvalue (`|SpawnActorFromClass` "/Game/ThirdPersonBP/Blueprints/ThirdPersonCharacter.ThirdPersonCharacter_C" (`self.GetTransform` (`self.K2_FindPlayerStart` NewPlayer (`KismetStringLibrary.Conv_IntToString` _array_index))) "AlwaysSpawn" "OverrideRootScale" null null))
          (if (== _array_index 0)
            (bind _tag (`/Game/ThirdPersonBP/Blueprints/ThirdPersonCharacter.Tag` _returnvalue))
            (`TextRenderComponent.K2_SetText` _tag "Instructor")
            (else
              (`TextRenderComponent.K2_SetText` _tag "Alumno")))
          (`Controller.Possess` _array_element _returnvalue))))))

(event `self.K2_OnLogout`
  (params (ExitingController :type "Controller Object Reference"))
  (bind _asplayer_controller (cast `PlayerController` ExitingController))
  (`KismetArrayLibrary.Array_RemoveItem` (`self.AllPlayers`) _asplayer_controller)
  (`KismetSystemLibrary.PrintString` "Removed succesful" true true (struct :`G` 0.66 :`B` 1.0 :`A` 1.0) 5.0))

(fn `UserConstructionScript`)